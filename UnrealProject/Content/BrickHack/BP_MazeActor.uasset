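; BP_MazeActor generates a maze from DimensionSizes and renders the part around the first-person player as a 2D slice along XAxis and YAxis.
; Each tick it converts the player's location to tile coordinates and gets neighboring cells within DisplayRadius.
; New cells add floor and wall mesh instances from GetWalls, while out-of-range cells have instances removed by sphere overlap.
; Start is never cleared here, and Cells is never pruned.
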(event EventBeginPlay
  (CallFunction|BuildMaze))

(event EventActorBeginOverlap
  (params (OtherActor :type Actor%20Object%20Reference)))

(event EventTick
  (params (DeltaSeconds :type Float%20%28single-precision%29))
  (Utilities|UpdateCellsatPlayer))

(fn ConstructionScript)

(fn BuildMaze
  (bind _dimensionsizes (Variables|MazeProperties|GetDimensionSizes))
  (bind _asfirst_person_character (Utilities|Casting|CastToFirstPersonCharacter (Game|GetPlayerCharacter 0)))
  (for _index (range 0 (- (Utilities|Array|Length _dimensionsizes) 1))
    (Utilities|Array|SetArrayElem (Utilities|Struct|BreakCoordinate (Variables|/Game/BrickHack/FirstPersonCharacter.FirstPersonCharacter_C|GetPosition _asfirst_person_character)) _index 0 true))
  (Variables|Default|SetStart true)
  (Class|MazeActor|GenerateMaze _dimensionsizes)
  (Utilities|UpdateCellsatPlayer))